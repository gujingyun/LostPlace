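; BP_LPEnemy is an enemy character Blueprint that handles spawn scaling, attack-facing warp targets and dissolve visuals.
; On BeginPlay, a timeline drives uniform mesh scale.
; UpdateFacingTarget feeds a location into Motion Warping as the FacingTarget warp target.
; StartDissolveTimeline plays a second timeline that writes the Dissolve scalar on every supplied dynamic material instance.
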(event EventBeginPlay
  (bind _新建轨道_1 (Timeline|时间轴 Play)
    (:Update
      (Transformation|SetRelativeScale3D (Variables|Character|GetMesh) (Math|Vector|MakeVector _新建轨道_1 _新建轨道_1 _新建轨道_1)))))

(event Collision|EventActorBeginOverlap
  (params (OtherActor :type Actor%20Object%20Reference)))

(event EventTick
  (params (DeltaSeconds :type Float%20%28single-precision%29)))

(event EventStartDissolveTimeline
  (params (DynamicMaterialInstance :type Array%20of%20Material%20Instance%20Dynamic%20Object%20References))
  (bind _dissolvetrack (Timeline|溶解时间轴 PlayFromStart)
    (:Update
      (for _array_element DynamicMaterialInstance
        (Rendering|Material|SetScalarParameterValue _array_element "Dissolve" _dissolvetrack :!class /Script/Engine.MaterialInstanceDynamic)))))

(event EventUpdateFacingTarget
  (params (Target :type Vector%20%28by%20ref%29 :default "0, 0, 0"))
  (Class|MotionWarpingComponent|AddorUpdateWarpTargetfromLocation (Variables|Default|GetMotionWarping) "FacingTarget" Target))

(fn ConstructionScript)