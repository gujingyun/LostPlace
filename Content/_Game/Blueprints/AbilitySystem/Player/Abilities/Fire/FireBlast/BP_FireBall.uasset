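; Fireball actor for the FireBlast ability that flies out along its forward vector, homes back to ReturnToActor and explodes on arrival.
; On authority, two chained timelines lerp its location without sweep, the return leg tracking the target's current position.
; Within ExplodeDistance it calls OnHit, applies radial damage effects to live players nearby except its owner, then destroys itself.
; Knockback points away from the blast with pitch overridden to 45 degrees.
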(event EventBeginPlay)

(event Collision|EventActorBeginOverlap
  (params (OtherActor :type Actor%20Object%20Reference)))

(event EventTick
  (params (DeltaSeconds :type Float%20%28single-precision%29)))

(event EventStartOutgoingTimeline
  (bind _returnvalue (Components|GetOwner))
  (bind _array (Utilities|Array|MakeArray _returnvalue))
  (Networking|SwitchHasAuthority
    (:Authority
      ;[0.15 0.11 0 0.5] 存储初始位置和顶点位置
      (Variables|Default|SetInitialLocation (Transformation|GetActorLocation))
      (Variables|Default|SetApexLocation (+ (Variables|Default|GetInitialLocation) (* (Transformation|GetActorForwardVector) (Variables|Default|GetTravelDistance))))
      (bind _outgoingtrack (Timeline|OutgoingTimeline Play)
        (:Update
          (Transformation|SetActorLocation (Math|Vector|Lerp(Vector) (Variables|Default|GetInitialLocation) (Variables|Default|GetApexLocation) _outgoingtrack) false false))
        (:Finished
          (bind _returningtrack (Timeline|ReturningTimeline Play)
            (:Update
              (Transformation|SetActorLocation (Math|Vector|Lerp(Vector) (Variables|Default|GetApexLocation) (Transformation|GetActorLocation (Variables|Default|GetReturnToActor)) _returningtrack) false false)
              (if (CallFunction|IsWithinExplodeDistance)
                (Class|Projectile|OnHit)
                (Utilities|Array|Add _array self)
                (bind _outoverlappingactors (Class|LPAbilitySystemLibrary|GetLivePlayersWithinRadius self _array (Variables|Default|GetRadialDamageOuterRadius) (Transformation|GetActorLocation)))
                (Variables|Default|SetOverlappingActors _outoverlappingactors)
                (Class|LPAbilitySystemLibrary|SetIsRadialDamageEffectParams (Variables|Default|GetExplosionDamageParams) true (Variables|Default|GetRadialDamageInnerRadius) (Variables|Default|GetRadialDamageOuterRadius) (Transformation|GetActorLocation))
                (for _array_element (Variables|Default|GetOverlappingActors)
                  (Class|LPAbilitySystemLibrary|SetEffectParamsTargetASC (Variables|Default|GetExplosionDamageParams) (Ability|GetAbilitySystemComponent _array_element))
                  (Variables|Default|SetKnockbackDirection (- (Transformation|GetActorLocation _array_element) (Transformation|GetActorLocation)))
                  (Class|LPAbilitySystemLibrary|SetKnockbackDirection (Variables|Default|GetExplosionDamageParams) (CallFunction|OverrideKnockbackPitch) (Variables|Default|GetKnockbackMagnitude))
                  (Class|LPAbilitySystemLibrary|SetDeathImpulseDirection (Variables|Default|GetExplosionDamageParams) (Variables|Default|GetKnockbackDirection) (Variables|Default|GetDeathImpulseMagnitude))
                  (Class|LPAbilitySystemLibrary|ApplyDamageEffect (Variables|Default|GetExplosionDamageParams)))
                (Actor|DestroyActor)))))))))

(fn ConstructionScript)

(fn IsWithinExplodeDistance
  (return (<= (Math|Vector|VectorLength (- (Transformation|GetActorLocation) (Transformation|GetActorLocation (Variables|Default|GetReturnToActor)))) (Variables|Default|GetExplodeDistance))))

(fn OverrideKnockbackPitch
  (bind _knockbackdirection (Variables|Default|GetKnockbackDirection))
  (bind _returnvalue (Math|Rotator|MakeRotfromX _knockbackdirection))
  (return (Math|Vector|GetForwardVector (Math|Rotator|MakeRotator (.roll _returnvalue) 45.0 (.yaw _returnvalue)))))