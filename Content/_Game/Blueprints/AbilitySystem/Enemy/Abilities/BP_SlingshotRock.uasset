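; BP_SlingshotRock is the rock actor for an enemy slingshot ability, giving the rock a random tumbling spin.
; On BeginPlay it runs the parent logic, then picks random signed yaw, pitch and roll rates.
; Tick applies those rates, scaled by delta time, as local rotation on the Rock component for a frame-rate independent tumble.
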(event EventBeginPlay
  (bind _returnvalue (Math|Random|RandomFloatinRange -5e+02 5e+02))
  (|CallParentFunction)
  (Variables|Default|SetYawRotatonRate _returnvalue)
  (Variables|Default|SetPitchRotatonRate _returnvalue)
  (Variables|Default|SetRollRotatonRate _returnvalue))

(event Collision|EventActorBeginOverlap
  (params (OtherActor :type Actor%20Object%20Reference)))

(event EventTick
  (params (DeltaSeconds :type Float%20%28single-precision%29))
  (Transformation|AddLocalRotation (Variables|Default|GetRock) (Math|Rotator|MakeRotator (* (Variables|Default|GetRollRotatonRate) DeltaSeconds) (* (Variables|Default|GetPitchRotatonRate) DeltaSeconds) (* DeltaSeconds (Variables|Default|GetYawRotatonRate))) false false))

(fn ConstructionScript)