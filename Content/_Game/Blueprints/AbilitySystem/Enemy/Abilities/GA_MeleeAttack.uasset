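; Enemy melee attack gameplay ability that faces the combat target and plays a random tagged attack montage.
; On the montage's gameplay event, it finds live players in a small sphere at the tagged combat socket and damages non-friends.
; A hit fires the MeleeImpact gameplay cue, then the ability ends.
; An IsAttacking flag blocks re-entry and clears only after that event, which is also awaited on interrupt or cancel.
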(event Ability|EventActivateAbility
  (bind _returnvalue (Ability|GetAvatarActorfromActorInfo))
  (bind _returnvalue_2 (Ability|GetAvatarActorfromActorInfo))
  (bind _returnvalue_3 (Ability|GetAvatarActorfromActorInfo))
  (if (not (Variables|Default|GetisAttacking))
    (Variables|Default|SetisAttacking true)
    (Variables|Default|SetHasHitTarget false)
    (bind _returnvalue_4 (Class|EnemyInterface|GetCombatTarget(Message) _returnvalue_3))
    (bind _ascombat_interface (Utilities|Casting|CastToCombatInterface _returnvalue_3))
    (Class|CombatInterface|UpdateFacingTarget _ascombat_interface (Transformation|GetActorLocation _returnvalue_4))
    (bind _returnvalue_5 (Class|CombatInterface|GetAttackMontages(Message) (Ability|GetAvatarActorfromActorInfo)))
    (bind _output_get (Variables|Default|SetTaggedMontage (Class|LPDamageGameplayAbility|GetRandomTaggedMontagefromArray _returnvalue_5)))
    (|PlayMontageandWaitProxy "None" (.Montage (Utilities|Struct|BreakTaggedMontage _output_get)) 1.0 "None" false 1.0 0.0 false
      (:then
        _)
      (:OnInterrupted
        _)
      (:OnCancelled
        _))
    (Ability|Tasks|WaitGameplayEvent (.MontageTag (Utilities|Struct|BreakTaggedMontage _output_get)) 0
      (:EventReceived
        (bind _returnvalue_6 (Class|CombatInterface|GetCombatSocketLocation(Message) _returnvalue_2 (.SocketTag (Utilities|Struct|BreakTaggedMontage _output_get))))
        (Variables|Default|SetCombatSocketLocation _returnvalue_6)
        (bind _outoverlappingactors (Class|LPAbilitySystemLibrary|GetLivePlayersWithinRadius _returnvalue_2 (Utilities|Array|MakeArray _returnvalue_2) 45.0 (Variables|Default|GetCombatSocketLocation)))
        (for _array_element _outoverlappingactors
          (if (Class|LPAbilitySystemLibrary|IsNotFriend (Ability|GetAvatarActorfromActorInfo) _array_element)
            (Class|LPDamageGameplayAbility|CauseDamage _array_element)
            (Variables|Default|SetHasHitTarget true)))
        (if (Variables|Default|GetHasHitTarget)
          (bind _returnvalue_7 (Class|EnemyInterface|GetCombatTarget(Message) _returnvalue))
          (Class|GameplayAbility|ExecuteGameplayCuewithParams "(TagName=\"GameplayCue.MeleeImpact\")" (Ability|GameplayCue|MakeGameplayCueParameters :AggregatedSourceTags (GameplayTags|MakeGameplayTagContainerfromTag (.MontageTag (Utilities|Struct|BreakTaggedMontage (Variables|Default|GetTaggedMontage)))) :Location (Variables|Default|GetCombatSocketLocation) :EffectCauser _returnvalue :SourceObject _returnvalue_7)))
        (Ability|EndAbility)
        (Variables|Default|SetisAttacking false)))))

(event Ability|EventOnEndAbility
  (params (bWasCancelled :type Boolean)))